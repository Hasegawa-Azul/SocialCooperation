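; BP_Panel is a puzzle panel that changes color on mouse hover while active, which a comment ties to Room1 being movable.
; The Panel component's cursor-over events swap its material between M_PanelON and M_PanelOFF.
; Both events are gated by IsActive, and a Highlighted flag prevents repeated swaps.
; Nothing in this graph sets IsActive, and BeginPlay, Tick and the construction script are empty.
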(event OnBeginCursorOver(Panel)
  (params (TouchedComponent :type Primitive%20Component%20Object%20Reference))
  ;[1 1 1] Room1が移動可能な時にマウスカーソルが重なった場合にRoom1の色が変化する処理
  (if (Variables|Default|GetIsActive)
    (if (not (Variables|Default|GetHighlighted))
      (Rendering|Material|SetMaterial (Variables|Default|GetPanel) 0 "/Game/PuzzleTest/Materials/M_PanelON.M_PanelON")
      (Variables|Default|SetHighlighted true))))

(event OnEndCursorOver(Panel)
  (params (TouchedComponent :type Primitive%20Component%20Object%20Reference))
  ;[1 1 1] Room1が移動可能な時にマウスカーソルが重なった場合にRoom1の色が変化する処理
  (if (Variables|Default|GetIsActive)
    (if (Variables|Default|GetHighlighted)
      (Rendering|Material|SetMaterial (Variables|Default|GetPanel) 0 "/Game/PuzzleTest/Materials/M_PanelOFF.M_PanelOFF")
      (Variables|Default|SetHighlighted false))))

(event EventBeginPlay)

(event Collision|EventActorBeginOverlap
  (params (OtherActor :type Actor%20Object%20Reference)))

(event EventTick
  (params (DeltaSeconds :type Float%20%28single-precision%29)))

(fn ConstructionScript)